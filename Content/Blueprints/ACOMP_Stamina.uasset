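; Stamina actor component that tracks and drains stamina for its owning Default_Players character.
; It caches its owner on BeginPlay.
; RefreshStamina subtracts the passed amount only while the character's movement velocity is non-zero, clamping the result between fixed bounds.
; Reaching zero sets the IsNotStamina flag, with no regeneration or flag reset in these graphs.
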(event `self.ReceiveBeginPlay`
  (set `self.Character` (`self.GetOwner`)))

(fn `RefreshStamina`
  (params (InStamina :type "Float (double-precision)"))
  (bind _asdefault_players (cast `/Game/Default_Players` (`self.Character`)))
  (if (> (`KismetMathLibrary.VSize` (`MovementComponent.Velocity` (`Character.CharacterMovement` _asdefault_players))) 0.0)
    (bind _output_get (set `self.Stamina` (`KismetMathLibrary.FClamp` (- (`self.Stamina`) InStamina) 0.0 100.0)))
    (if (== _output_get 0.0)
      (set `self.IsNotStamina` true)
      (return))))