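; ACOMP_TIME is an in-game clock and calendar that tracks time of day and date.
; BeginPlay seeds a float CLOCK from the time fields; each unpaused Tick advances it by delta time divided by TimeMultiplier, wrapping at 24.
; Hour, minute and second derive from CLOCK, while wrap counts feed day, month and year rollover using DaysInMonth.
; The current time and date print on screen every unpaused frame.
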(event `self.ReceiveBeginPlay`
  (set `self.CLOCK` (+ (`KismetMathLibrary.Conv_IntToDouble` (`self.Second`)) (`KismetMathLibrary.Conv_IntToDouble` (/ (`self.Minute`) 60)) (`KismetMathLibrary.Conv_IntToDouble` (/ (`self.Hour`) 24)))))

(event `self.ReceiveTick`
  (params (DeltaSeconds :type "Float (single-precision)"))
  (bind (_remainder _returnvalue) (`KismetMathLibrary.FMod` (* (`self.CLOCK`) 3600.0) 60.0))
  (bind (_remainder_2 _returnvalue_2) (`KismetMathLibrary.FMod` (+ (/ DeltaSeconds (`self.TimeMultiplier`)) (`self.CLOCK`)) 24.0))
  (bind (_remainder_3 _returnvalue_3) (`KismetMathLibrary.FMod` (`KismetMathLibrary.Conv_IntToDouble` _returnvalue) 60.0))
  (if (not (`self.IS_Pause?`))
    (set `self.CLOCK` _remainder_2)
    (set `self.DayTick` _returnvalue_2)
    ;[1 1 1] Second
    (set `self.Second` (`KismetMathLibrary.FFloor` _remainder))
    ;[1 1 1] Minute
    (set `self.Minute` (`KismetMathLibrary.FFloor` _remainder_3))
    ;[1 1 1] Hour
    (set `self.Hour` (`KismetMathLibrary.FFloor` (`KismetMathLibrary.FMod` (`KismetMathLibrary.Conv_IntToDouble` _returnvalue_3) 24.0)))
    (bind _output_get (set `self.Day` (+ (`self.Day`) (`self.DayTick`))))
    (if (> _output_get (`KismetMathLibrary.DaysInMonth` (`self.Year`) (`self.Month`)))
      (set `self.Day` 1)
      (`/Engine/EditorBlueprintResources/StandardMacros.IncrementInt` (`self.Month`)
        (:`  `
          _)))
    (if (> (`self.Month`) 12)
      (set `self.Month` 1)
      (`/Engine/EditorBlueprintResources/StandardMacros.IncrementInt` (`self.Year`)
        (:`  `
          _)))
    (`KismetSystemLibrary.PrintString` (`KismetStringLibrary.Concat_StrStr` (`KismetStringLibrary.Concat_StrStr` (`KismetTextLibrary.Conv_TextToString` (`KismetTextLibrary.Conv_IntToText` (`self.Hour`) true 2 2)) ":" (`KismetTextLibrary.Conv_TextToString` (`KismetTextLibrary.Conv_IntToText` (`self.Minute`) true 2 2)) ":" (`KismetTextLibrary.Conv_TextToString` (`KismetTextLibrary.Conv_IntToText` (`self.Second`) true 2 2))) " - " (`KismetStringLibrary.Concat_StrStr` (`KismetTextLibrary.Conv_TextToString` (`KismetTextLibrary.Conv_IntToText` (`self.Day`) true 2 2)) "/" (`KismetTextLibrary.Conv_TextToString` (`KismetTextLibrary.Conv_IntToText` (`self.Month`) true 2 2)) "/" (`KismetStringLibrary.Conv_IntToString` (`self.Year`)))) true true (struct :`R` 1.0 :`G` 0.958534 :`B` 0.011733 :`A` 1.0) 0.0)))