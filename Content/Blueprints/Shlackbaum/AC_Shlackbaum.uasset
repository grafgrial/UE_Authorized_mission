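; AC_Shlackbaum is an interactive boom barrier (Schlagbaum) that the player raises with E and that lowers itself afterwards.
; Its box trigger enables input and opens a gate node for overlapping actors implementing BPI_Interact_Signal, letting E open a closed barrier.
; A Timeline rotates the boom, playing or reversing by IsOpen, which flips on completion.
; Leaving the box disables input and, if open, closes the barrier after a short delay.
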(event `Open_Shlackbaum`
  (if (`self.Is Open?`)
    (bind (_direction _alpha_rotation) (`Timeline|Timeline_0` :!via `Reverse` :!label _label)
      (:`Update`
        (`SceneComponent.K2_SetRelativeRotation` (`self.Shlackbaum_Cube_001`) (`KismetMathLibrary.RLerp` (struct) (struct :`Pitch` -55.0) _alpha_rotation) false false))
      (:`Finished`
        (if (`self.Is Open?`)
          (set `self.Is Open?` false)
          (else
            (set `self.Is Open?` true)))))
    (else
      (goto _label))))

(event `Key|E`
  (params (Key :type "Key Structure" :default "AnyKey"))
  (:`Pressed`
    (`/Engine/EditorBlueprintResources/StandardMacros.Gate` true :!label _label_2
      (:`Exit`
        (if (not (`self.Is Open?`))
          (`self.Open_Shlackbaum`))))))

(event `self.Box.OnComponentBeginOverlap`
  (params (OverlappedComponent :type "PrimitiveComponent Object Reference") (OtherActor :type "Actor Object Reference") (OtherComp :type "PrimitiveComponent Object Reference") (OtherBodyIndex :type Integer) (bFromSweep :type Boolean) (SweepResult :type "HitResult Structure (by ref)"))
  (if (`KismetSystemLibrary.DoesImplementInterface` OtherActor "/Game/Blueprints/BPI_Interact_Signal.BPI_Interact_Signal_C")
    (`self.EnableInput` (`GameplayStatics.GetPlayerController` 0))
    (goto _label_2 :!via `Open`)))

(event `self.Box.OnComponentEndOverlap`
  (params (OverlappedComponent :type "PrimitiveComponent Object Reference") (OtherActor :type "Actor Object Reference") (OtherComp :type "PrimitiveComponent Object Reference") (OtherBodyIndex :type Integer))
  (if (`KismetSystemLibrary.DoesImplementInterface` OtherActor "/Game/Blueprints/BPI_Interact_Signal.BPI_Interact_Signal_C")
    (if (`self.Is Open?`)
      (`KismetSystemLibrary.Delay` 0.5)
      (`self.Open_Shlackbaum`))
    (`self.DisableInput` (`GameplayStatics.GetPlayerController` 0))
    (goto _label_2 :!via `Close`)))

(fn `UserConstructionScript`)