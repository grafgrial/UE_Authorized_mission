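; Alarm button that toggles a shared alarm (trevoga) signal and shows it with a flashing point light.
; InteractSignal starts or stops the alarm from the current Status and reports it to TopDownGameMode, whose bound signal event updates Status through RefreshSignal.
; Server-named events call client-named ones, which drive light intensity with a timeline or zero it.
; Box overlap only prints interactors' names and clears the character reference.
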(event `self.ReceiveBeginPlay`
  (bind _astop_down_game_mode (cast `/Game/TopDownBP/Blueprints/TopDownGameMode` (`GameplayStatics.GetGameMode`)))
  (bind _output_get (set `self.GameMode` _astop_down_game_mode))
  (add `/Game/TopDownBP/Blueprints/TopDownGameMode.signalss` _output_get (delegate `ser`)))

(event `ser`
  (params (issiganl :type Boolean))
  (`self.RefreshSignal` issiganl))

(event `TREVOGA_Server`
  (`self.TREVOGA_Client`))

(event `TREVOGA_Client`
  (bind (_direction _loop) (`Timeline|Timeline_0` :!label _label)
    (:`Update`
      (`LightComponent.SetIntensity` (`self.PointLight`) (`KismetMathLibrary.Lerp` 0.0 5000.0 _loop)))))

(event `Stop`
  (goto _label :!via `Stop`))

(event `NOtrevoraSERVER`
  (`self.NOtrevogaClient`))

(event `NOtrevogaClient`
  (`LightComponent.SetIntensity` (`self.PointLight`) 0.0)
  (`self.Stop`))

(event `self.Box.OnComponentBeginOverlap`
  (params (OverlappedComponent :type "PrimitiveComponent Object Reference") (OtherActor :type "Actor Object Reference") (OtherComp :type "PrimitiveComponent Object Reference") (OtherBodyIndex :type Integer) (bFromSweep :type Boolean) (SweepResult :type "HitResult Structure (by ref)"))
  (if (`KismetSystemLibrary.DoesImplementInterface` OtherActor "/Game/Blueprints/BPI_Interact_Signal.BPI_Interact_Signal_C")
    (`KismetSystemLibrary.PrintString` (`KismetSystemLibrary.GetDisplayName` OtherActor))
    (set `self.REF_Character` null)))

(event `self.Box.OnComponentEndOverlap`
  (params (OverlappedComponent :type "PrimitiveComponent Object Reference") (OtherActor :type "Actor Object Reference") (OtherComp :type "PrimitiveComponent Object Reference") (OtherBodyIndex :type Integer))
  (set `self.REF_Character` null))

(fn `InteractSignal`
  (params (Player :type "Character Object Reference"))
  (returns (NewParam :type "Character Object Reference"))
  (bind _gamemode (`self.GameMode`))
  (if (`self.status`)
    (`self.NOtrevoraSERVER`)
    (`/Game/TopDownBP/Blueprints/TopDownGameMode.SetStat` _gamemode false)
    (else
      (`self.TREVOGA_Server`)
      (`/Game/TopDownBP/Blueprints/TopDownGameMode.SetStat` _gamemode true)))
  (return null))

(fn `RefreshSignal`
  (params (IsSignal :type Boolean))
  (bind _output_get (set `self.Status` IsSignal))
  (if _output_get
    (`self.TREVOGA_Server`)
    (else
      (`self.NOtrevoraSERVER`))))

(fn `UserConstructionScript`)