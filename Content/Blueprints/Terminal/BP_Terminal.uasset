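; Interactable terminal that toggles an alarm ("trevoga") and shows it with a spotlight.
; InteractSignal flips the alarm flag stored in the GameMode, and BeginPlay applies the current flag to the light.
; Server-named events forward to client-named events, which either run a timeline driving red light intensity or stop it and switch the light off.
; Box overlaps only clear the stored character reference and print the name of interface-implementing actors.
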(event `TREVOGA_Client`
  (bind (_direction _loop) (`Timeline|Timeline_0` :!label _label)
    (:`Update`
      (`LightComponent.SetIntensity` (`self.SpotLight`) (`KismetMathLibrary.Lerp` 0.0 5000.0 _loop))
      (`LightComponent.SetLightColor` (`self.SpotLight`) (struct :`R` 1.0 :`A` 1.0) true))))

(event `TREVOGA_Server`
  (`self.TREVOGA_Client`))

(event `Stop`
  (goto _label :!via `Stop`))

(event `self.ReceiveBeginPlay`
  (`self.RefreshTREVOGA`))

(event `NOtrevoraSERVER`
  (`self.NOtrevogaClient`))

(event `NOtrevogaClient`
  (`LightComponent.SetLightColor` (`self.SpotLight`) (struct :`R` 1.0 :`G` 1.0 :`B` 1.0 :`A` 1.0) true)
  (`LightComponent.SetIntensity` (`self.SpotLight`) 0.0)
  (`self.Stop`))

(event `self.Box.OnComponentBeginOverlap`
  (params (OverlappedComponent :type "PrimitiveComponent Object Reference") (OtherActor :type "Actor Object Reference") (OtherComp :type "PrimitiveComponent Object Reference") (OtherBodyIndex :type Integer) (bFromSweep :type Boolean) (SweepResult :type "HitResult Structure (by ref)"))
  (if (`KismetSystemLibrary.DoesImplementInterface` OtherActor "/Game/Blueprints/BPI_Interact_Signal.BPI_Interact_Signal_C")
    (`KismetSystemLibrary.PrintString` (`KismetSystemLibrary.GetDisplayName` OtherActor))
    (set `self.REF_Character` null)))

(event `self.Box.OnComponentEndOverlap`
  (params (OverlappedComponent :type "PrimitiveComponent Object Reference") (OtherActor :type "Actor Object Reference") (OtherComp :type "PrimitiveComponent Object Reference") (OtherBodyIndex :type Integer))
  (set `self.REF_Character` null))

(fn `GETstatus`
  (returns (Status :type Boolean))
  (return false))

(fn `InteractSignal`
  (params (Player :type "Character Object Reference"))
  (returns (NewParam :type "Character Object Reference"))
  (bind _returnvalue (`GameplayStatics.GetGameMode`))
  (set `self.REF_Character` Player)
  (bind _status (`self.RefreshTREVOGA`))
  (if _status
    (message `/Game/Blueprints/BPI_Sig.SetStat` _returnvalue false)
    (`self.NOtrevoraSERVER`)
    (`KismetSystemLibrary.PrintString` "notr")
    (else
      (message `/Game/Blueprints/BPI_Sig.SetStat` _returnvalue true)
      (`self.TREVOGA_Server`)
      (`KismetSystemLibrary.PrintString` "tr")))
  (return null))

(fn `RefreshTREVOGA`
  (returns (Status :type Boolean))
  (bind _newparam (message `/Game/Blueprints/BPI_Sig.GetStat` (`GameplayStatics.GetGameMode`)))
  (if _newparam
    (`self.TREVOGA_Server`)
    (return true)
    (else
      (`self.NOtrevoraSERVER`)
      (return false))))

(fn `UserConstructionScript`)