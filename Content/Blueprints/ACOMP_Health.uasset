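; Health component that tracks a Health value up to HealthMax, with restore, damage and optional timed regeneration.
; RestoreHealth clamps at the maximum, while RemoveHealth triggers Death on lethal damage, firing a dispatcher without setting Health to zero.
; When IsRegen is set, a looping timer adds health, pauses itself at full and is unpaused by non-lethal damage.
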(event `self.ReceiveBeginPlay`
  (if (`self.Is Regen?`)
    (bind _returnvalue (`KismetSystemLibrary.K2_SetTimer` null "RegenerationHealth" (`self.RegenRate`) true))
    (set `self.TimerRegen` _returnvalue)))

(event `Death`
  (`self.DISP_Death`))

(fn `RegenerationHealth`
  (bind _returnvalue (+ (`self.Health`) (`self.RegenAmounts`)))
  (if (`self.Is Regen?`)
    (if (>= _returnvalue (`self.Health_Max`))
      (set `self.Health` (`self.Health_Max`))
      (`KismetSystemLibrary.K2_PauseTimerHandle` (`self.TimerRegen`))
      (else
        (set `self.Health` _returnvalue)))))

(fn `RemoveHealth`
  (params (AmountToRemove :type "Float (double-precision)"))
  (bind _returnvalue (- (`self.Health`) AmountToRemove))
  (if (<= _returnvalue 0.0)
    (`self.Death`)
    (else
      (set `self.Health` _returnvalue)
      (if (< (`self.Health`) (`self.Health_Max`))
        (`KismetSystemLibrary.K2_UnPauseTimerHandle` (`self.TimerRegen`))))))

(fn `RestoreHealth`
  (params (AmountToRestore :type "Float (double-precision)"))
  (bind _returnvalue (+ (`self.Health`) AmountToRestore))
  (if (>= _returnvalue (`self.Health_Max`))
    (set `self.Health` (`self.Health_Max`))
    (else
      (set `self.Health` _returnvalue))))