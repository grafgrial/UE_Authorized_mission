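; BP_Signal is an alarm siren actor (TREVOGA means alarm) that starts and stops an Audio component.
; Server-named events forward to client-named events that play the sound with a fade-in, or fade it out.
; The stop event calls Stop immediately after FadeOut, so the fade is cut short.
; BeginPlay calls RefreshTREVOGA, which reads a stat message from the GameMode but does nothing with it.
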(event `self.ReceiveBeginPlay`
  (`self.RefreshTREVOGA`))

(event `TREVOGA_Client`
  (bind _audio (`self.Audio`))
  (`AudioComponent.Play` _audio 0.0)
  (`AudioComponent.FadeIn` _audio 2.0 1.0 0.0))

(event `TREVOGA_Server`
  (`self.TREVOGA_Client`))

(event `NOtrevoraSERVER`
  (`self.NOtrevogaClient`))

(event `NOtrevogaClient`
  (bind _audio (`self.Audio`))
  (`AudioComponent.FadeOut` _audio 2.0 0.0)
  (`AudioComponent.Stop` _audio))

(fn `RefreshTREVOGA`
  (bind _newparam (message `/Game/Blueprints/BPI_Sig.GetStat` (`GameplayStatics.GetGameMode`)))
  (if _newparam
    _))

(fn `UserConstructionScript`)