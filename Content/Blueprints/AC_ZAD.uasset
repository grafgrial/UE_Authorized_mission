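; Test actor that detects when the player is behind it, printing "Сзади" ("Behind") as debug output.
; A Box begin overlap calls Goor, which takes the dot product of the direction to player 0 and the actor's rotation X axis, treating negative as behind.
; The overlap guard only checks player controller 0, not the overlapping actor, so other overlaps also trigger the test.
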(event `Goor`
  (if (< (`KismetMathLibrary.Dot_VectorVector` (`KismetMathLibrary.Normal` (- (`self.K2_GetActorLocation` (`GameplayStatics.GetPlayerCharacter` 0)) (`self.K2_GetActorLocation`))) (`KismetMathLibrary.Normal` (`KismetMathLibrary.BreakRotIntoAxes` (`self.K2_GetActorRotation`)))) 0.0)
    (`KismetSystemLibrary.PrintString` "Сзади")))

(event `self.Box.OnComponentBeginOverlap`
  (params (OverlappedComponent :type "PrimitiveComponent Object Reference") (OtherActor :type "Actor Object Reference") (OtherComp :type "PrimitiveComponent Object Reference") (OtherBodyIndex :type Integer) (bFromSweep :type Boolean) (SweepResult :type "HitResult Structure (by ref)"))
  (if (`Controller.IsPlayerController` (`GameplayStatics.GetPlayerController` 0))
    (`self.Goor`)))

(event `self.Box.OnComponentEndOverlap`
  (params (OverlappedComponent :type "PrimitiveComponent Object Reference") (OtherActor :type "Actor Object Reference") (OtherComp :type "PrimitiveComponent Object Reference") (OtherBodyIndex :type Integer)))

(fn `UserConstructionScript`)